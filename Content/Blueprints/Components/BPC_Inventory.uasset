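; BPC_Inventory is an inventory component that stores ingredient structs in an array.
; BeginPlay resizes the array to InventorySize, though adding an item appends past those default slots instead of filling them.
; Removal deletes the first matching entry, and both add and remove call OnInventoryChanged to signal the change.
; A debug function prints each slot's index and ingredient name.
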(event EventBeginPlay
  (Utilities|Array|Resize (Variables|Default|GetSIngredientInventory) (Variables|Default|GetInventorySize)))

(event EventTick
  (params (DeltaSeconds :type Float%20%28single-precision%29)))

(fn RemoveItemUsed
  (params (ItemToFind :type S%20Ingredient%20Structure%20%28by%20ref%29))
  (bind _singredientinventory (Variables|Default|GetSIngredientInventory))
  (Utilities|Array|RemoveIndex _singredientinventory (Utilities|Array|FindItem _singredientinventory ItemToFind))
  (Default|CallOnInventoryChanged))

(fn AddItemtoInventory
  (params (NewItem :type S%20Ingredient%20Structure%20%28by%20ref%29))
  (Utilities|Array|Add (Variables|Default|GetSIngredientInventory) NewItem)
  (Default|CallOnInventoryChanged))

(fn PrintInventory
  (for (_array_element _array_index) (Variables|Default|GetSIngredientInventory)
    (Development|PrintString (Utilities|String|Append (Utilities|String|ToString(Integer) _array_index) ":" (Utilities|String|ToString(Text) (.Name (Utilities|Struct|BreakSIngredient _array_element)))))))