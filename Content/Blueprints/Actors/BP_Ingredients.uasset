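; BP_Ingredients is a pickup actor for an ingredient the player can collect into their inventory.
; On BeginPlay it caches the BP_Player pawn and looks up its IngredientID row in DT_Ingredients to set the floating 3D name text, mesh and material.
; Interacting adds that ingredient data to the player's BPCInventory component and destroys the actor.
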(event EventBeginPlay
  (bind _ingredient (Variables|Default|GetIngredient))
  ;[0.15 0.15 0.15 0.5] A
  (bind _asbp_player (Utilities|Casting|CastToBP_Player (Game|Player|GetPlayerPawn 0)))
  (Variables|Default|SetAs%20BP%20Player _asbp_player)
  ;[0.15 0.15 0.15 0.5] Assign the ingredient with his data table
  (bind _returnvalue (Utilities|GetDataTableRow "/Game/Data/Datatables/DT_Ingredients.DT_Ingredients" (Variables|Default|GetIngredientID))
    (:then
      (Variables|Default|SetIngredientData _returnvalue)
      (Rendering|Components|TextRender|SetText (Variables|Default|Get3DTextName) (Utilities|Text|ToText(String) (.name (Variables|Default|GetIngredientData))))
      (Components|StaticMesh|SetStaticMesh _ingredient (.mesh (Variables|Default|GetIngredientData)))
      (Rendering|Material|SetMaterial _ingredient 0 (.texture (Variables|Default|GetIngredientData))))))

(event Collision|EventActorBeginOverlap
  (params (OtherActor :type Actor%20Object%20Reference)))

(event EventTick
  (params (DeltaSeconds :type Float%20%28single-precision%29)))

(event EventInteract
  (Default|AddItemtoInventory (Variables|/Game/Blueprints/Actors/BP_Player.BP_Player_C|GetBPC_Inventory (Variables|Default|GetAs%20BP%20Player)) (Variables|Default|GetIngredientData))
  (Actor|DestroyActor))

(fn ConstructionScript)