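; BP_Workbench is an interactable station meant for cutting or grinding the player's selected ingredient.
; Interact switches to UI-only input focused on the workbench widget, though that widget's creation is disconnected.
; TransformIngredient passes Cut or Grind to ProcessIngredients, which currently only prints a warning for already processed ingredients.
; The logic building the renamed ingredient, updating inventory and closing the widget is present but unconnected.
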(event Custom|TransformIngredient
  (bind _method (Variables|Default|GetMethod))
  (switch Utilities|FlowControl|Switch|SwitchonEProcessingMethod _method
    (:NewEnumerator0
      _)
    (:NewEnumerator1
      _))
  (CallFunction|ProcessIngredients (Variables|/Game/Widgets/HUD/WBP_Inventory.WBP_Inventory_C|GetSelectedIngredient (Variables|/Game/Blueprints/Actors/BP_Player.BP_Player_C|GetInventory (Variables|Default|GetAs%20BP%20Player))) _method))

(event EventBeginPlay
  (bind _asbp_player (Utilities|Casting|CastToBP_Player (Game|Player|GetPlayerPawn 0)))
  (Variables|Default|SetAs%20BP%20Player _asbp_player))

(event EventInteract
  (params (Interactor :type BP%20Player%20Object%20Reference))
  (bind _as_bp_player (Variables|Default|GetAs%20BP%20Player))
  (bind _as_player_controller (Variables|/Game/Blueprints/Actors/BP_Player.BP_Player_C|GetAs%20Player%20Controller _as_bp_player))
  (if (Variables|Default|GetWidgetBoolean)
    (Variables|/Script/Engine.PlayerController|SetbShowMouseCursor _as_player_controller true)
    (Variables|Default|SetWidgetBoolean false)
    (Input|SetInputModeUIOnly _as_player_controller (Variables|Default|GetWBPWorkbench) "DoNotLock" false)))

(fn ConstructionScript)

(fn ProcessIngredients
  (params (InIngredient :type S%20Ingredient%20Structure) (Method :type EProcessingMethod%20Enum :default "NewEnumerator0"))
  (if (.IngredientTransform (Utilities|Struct|BreakSIngredient InIngredient))
    (Development|PrintString "Ingredient already process")))

(fn FocusTarget
  (return ""))