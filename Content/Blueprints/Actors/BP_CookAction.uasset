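; Possessable potion-crafting workbench that acts as a cutting station, grinder or cauldron according to Method, which also sets its mesh.
; Interact possesses it and binds inventory selection, and Escape returns control to BP_Player.
; Cut and Grind swap raw ingredients for transformed ones, each keeping a different property.
; The cauldron consumes transformed ingredients into a property-count map, compares it exactly against DT_Recipes, and only prints the resulting potion.
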(event Custom|LaunchCauldron
  ;[0.15 0.15 0.15 0.5] Système de craft de potion
  (bind _outrownames (DataTable|GetDataTableRowNames (Variables|Default|GetDT_Recipes)))
  (bind _array_element (Utilities|Array|ForEachLoopwithBreak _outrownames :!label _label)
    (:LoopBody
      (bind _returnvalue (Utilities|GetDataTableRow "/Game/Data/Datatables/DT_Recipes.DT_Recipes" _array_element)
        (:then
          (if (CallFunction|CompareMap (Variables|Default|GetTempProperty) (.ingredients _returnvalue))
            (Utilities|Map|Clear (Variables|Default|GetTempProperty))
            (Development|PrintString (Utilities|String|ToString(Name) (.resultingpotion _returnvalue)))
            (goto _label Break)))))))

(event Custom|ProcessIngredient
  (bind _as_bp_player (Variables|Default|GetAs%20BP%20Player))
  (bind _inventory (Variables|/Game/Blueprints/Actors/BP_Player.BP_Player_C|GetInventory _as_bp_player))
  (bind _selectedingredient (Variables|/Game/Widgets/HUD/WBP_Inventory.WBP_Inventory_C|GetSelectedIngredient _inventory))
  (switch Utilities|FlowControl|Switch|SwitchonEProcessingMethod (Variables|Default|GetMethod)
    (:NewEnumerator0
      (if (Utilities|Array|ContainsItem (Variables|/Game/Blueprints/Components/BPC_Inventory.BPC_Inventory_C|GetSIngredientInventory (Variables|/Game/Blueprints/Actors/BP_Player.BP_Player_C|GetBPC_Inventory _as_bp_player)) _selectedingredient) :!label _label
        (Development|PrintString "Process")
        (CallFunction|ProcessIngredients _selectedingredient (Variables|Default|GetMethod))
        (else
          (Development|PrintString "No item select"))))
    (:NewEnumerator1
      (goto _label))
    (:NewEnumerator2
      (if (.IngredientTransform (Utilities|Struct|BreakSIngredient _selectedingredient))
        (CallFunction|AddIngredientTemp _selectedingredient)
        (else
          (Development|PrintString "Ingredient not Process"))))))

(event Input|EnhancedActionEvents|EnhancedInputActionIA_EscapeWorkbench
  (params (ActionValue :type Boolean) (ElapsedSeconds :type Float%20%28double-precision%29) (TriggeredSeconds :type Float%20%28double-precision%29) (InputAction :type Input%20Action%20Object%20Reference :default "/Game/FirstPerson/Input/Actions/IA_EscapeWorkbench.IA_EscapeWorkbench"))
  (bind _as_bp_player (Variables|Default|GetAs%20BP%20Player))
  (bind _as_player_controller (Variables|/Game/Blueprints/Actors/BP_Player.BP_Player_C|GetAs%20Player%20Controller _as_bp_player))
  (Pawn|Possess _as_player_controller _as_bp_player)
  (Variables|/Script/Engine.PlayerController|SetbShowMouseCursor _as_player_controller false)
  (EventDispatchers|UnbindEventfromIngredientSelect (Variables|/Game/Blueprints/Actors/BP_Player.BP_Player_C|GetInventory (Variables|Default|GetAs%20BP%20Player)) (EventDispatchers|CreateEvent :!event Custom|ProcessIngredient))
  (switch Utilities|FlowControl|Switch|SwitchonEProcessingMethod (Variables|Default|GetMethod)
    (:NewEnumerator2
      (Widget|RemovefromParent (Variables|Default|GetWidgetCauldron)))))

(event EventBeginPlay
  (bind _meshworkbench (Variables|Default|GetMeshWorkbench))
  (bind _meshworkbench_2 (Variables|Default|GetMeshWorkbench))
  (bind _asbp_player (Utilities|Casting|CastToBP_Player (Game|Player|GetPlayerPawn 0)))
  (Variables|Default|SetAs%20BP%20Player _asbp_player)
  (switch Utilities|FlowControl|Switch|SwitchonEProcessingMethod (Variables|Default|GetMethod)
    (:NewEnumerator0
      (Components|StaticMesh|SetStaticMesh _meshworkbench "/Game/Fantastic_Village_Pack/meshes/props/deco/SM_PROP_knife_01.SM_PROP_knife_01")
      (Rendering|Material|SetMaterial _meshworkbench 0 "/Game/Fantastic_Village_Pack/materials/MI_metal_02.MI_metal_02")
      (Rendering|Material|SetMaterial _meshworkbench 1 "/Game/Fantastic_Village_Pack/materials/MI_wood_planks_07.MI_wood_planks_07"))
    (:NewEnumerator1
      (Components|StaticMesh|SetStaticMesh _meshworkbench "/Game/Fantastic_Village_Pack/meshes/props/food/SM_PROP_bowl_metal.SM_PROP_bowl_metal")
      (Rendering|Material|SetMaterial _meshworkbench 0 "/Game/Fantastic_Village_Pack/materials/MI_metal_01.MI_metal_01"))
    (:NewEnumerator2
      (Transformation|SetWorldLocation _meshworkbench_2 (- (Transformation|GetWorldLocation _meshworkbench_2) "0.000000,0.000000,50.000000") false true)
      (Components|StaticMesh|SetStaticMesh _meshworkbench "/Game/Fantastic_Village_Pack/meshes/props/food/SM_PROP_cookingpot_big.SM_PROP_cookingpot_big")
      (Rendering|Material|SetMaterial _meshworkbench 0 "/Game/Fantastic_Village_Pack/materials/MI_metal_01.MI_metal_01")
      (Rendering|Material|SetMaterial _meshworkbench 1 "/Game/Fantastic_Village_Pack/materials/MI_PROP_food.MI_PROP_food"))))

(event EventInteract
  (bind _as_bp_player (Variables|Default|GetAs%20BP%20Player))
  (bind _as_player_controller (Variables|/Game/Blueprints/Actors/BP_Player.BP_Player_C|GetAs%20Player%20Controller _as_bp_player))
  (Pawn|Possess _as_player_controller self)
  (Variables|/Script/Engine.PlayerController|SetbShowMouseCursor _as_player_controller true)
  (EventDispatchers|BindEventtoIngredientSelect (Variables|/Game/Blueprints/Actors/BP_Player.BP_Player_C|GetInventory (Variables|Default|GetAs%20BP%20Player)) (EventDispatchers|CreateEvent :!event Custom|ProcessIngredient))
  (switch Utilities|FlowControl|Switch|SwitchonEProcessingMethod (Variables|Default|GetMethod)
    (:NewEnumerator2
      (bind _returnvalue (UserInterface|CreateWidget "/Game/Widgets/HUD/WBP_Caudron.WBP_Caudron_C"))
      (bind _output_get (Variables|Default|SetWidgetCauldron _returnvalue))
      (UserInterface|Viewport|AddtoViewport _output_get 0)
      (EventDispatchers|BindEventtoOnClickProcess (Variables|Default|GetWidgetCauldron) (EventDispatchers|CreateEvent :!event Custom|LaunchCauldron)))))

(fn ConstructionScript)

(fn ProcessIngredients
  (params (InIngredient :type S%20Ingredient%20Structure) (Method :type EProcessingMethod%20Enum :default "NewEnumerator0"))
  (bind (_name _property1 _property2 _id _ingredienttransform _finalproperty _mesh _texture) (Utilities|Struct|BreakSIngredient InIngredient))
  (bind _as_bp_player (Variables|Default|GetAs%20BP%20Player))
  (bind _bpc_inventory (Variables|/Game/Blueprints/Actors/BP_Player.BP_Player_C|GetBPC_Inventory _as_bp_player))
  (if _ingredienttransform
    (Development|PrintString "Ingredient already process")
    (else
      (Default|AddItemtoInventory _bpc_inventory (Utilities|Select :Index Method :NewEnumerator0 (Utilities|Struct|MakeSIngredient (Utilities|String|Append _name " decoupe") _property1 _property2 _id true _property1 _mesh _texture) :NewEnumerator1 (Utilities|Struct|MakeSIngredient (Utilities|String|Append _name " moulu") _property1 _property2 _id true _property2 _mesh _texture) :NewEnumerator2 ""))
      (Default|RemoveItemUsed _bpc_inventory (Variables|/Game/Widgets/HUD/WBP_Inventory.WBP_Inventory_C|GetSelectedIngredient (Variables|/Game/Blueprints/Actors/BP_Player.BP_Player_C|GetInventory _as_bp_player))))))

(fn CompareMap
  (params (MapA_Ingredient :type Map%20of%20Strings%20to%20Integers) (MapB_Recipe :type Map%20of%20Strings%20to%20Integers))
  (if (== (Utilities|Map|Length MapA_Ingredient) (Utilities|Map|Length MapB_Recipe))
    (bind _keys (Utilities|Map|Keys MapA_Ingredient))
    (for _array_element _keys
      (if (Utilities|Map|Contains MapB_Recipe _array_element)
        (if (== (.Value (Utilities|Map|Find MapA_Ingredient _array_element)) (.Value (Utilities|Map|Find MapB_Recipe _array_element)))
          (Variables|Default|SetIs%20Matching true)
          (else
            (return false)))
        (else
          (return false))))
    (return true)
    (else
      (return false))))

(fn AddIngredientTemp
  (params (IngredientIn :type S%20Ingredient%20Structure))
  (bind _as_bp_player (Variables|Default|GetAs%20BP%20Player))
  (bind _bpc_inventory (Variables|/Game/Blueprints/Actors/BP_Player.BP_Player_C|GetBPC_Inventory _as_bp_player))
  (if (Utilities|Array|IsNotEmpty (Variables|/Game/Blueprints/Components/BPC_Inventory.BPC_Inventory_C|GetSIngredientInventory _bpc_inventory))
    (if true
      (for _array_element (Utilities|Array|MakeArray (.FinalProperty (Utilities|Struct|BreakSIngredient IngredientIn)))
        (if (Utilities|Map|Contains (Variables|Default|GetTempProperty) _array_element)
          (bind _result (Math|Integer|IncrementInt (.Value (Utilities|Map|Find (Variables|Default|GetTempProperty) _array_element)))
            (:%20%20
              (Utilities|Map|Add (Variables|Default|GetTempProperty) _array_element _result)))
          (else
            (Utilities|Map|Add (Variables|Default|GetTempProperty) _array_element 1))))
      (bind _output_get (Variables|Default|SetTempProperty (Variables|Default|GetTempProperty)))
      (bind _keys (Utilities|Map|Keys _output_get))
      (for _array_element_2 _keys
        (Development|PrintString _array_element_2))
      (Default|RemoveItemUsed _bpc_inventory IngredientIn)
      (else
        (Development|PrintString "Impossibe ingredient brute")))
    (else
      (Development|PrintString "No Ingredient in inventory"))))